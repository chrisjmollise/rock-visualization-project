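; RockBP is a rock actor that randomizes its mesh, material and color index, and avoids sharing a color with rocks it touches.
; Construction prepares a colored dynamic instance of RockMat_Inst but displays a random mesh material.
; A mask dispatcher event, bound on BeginPlay, swaps in the colored instance.
; Hit or overlap with another RockBP of the same color index re-rolls the color, which can repeat.
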(event `self.ReceiveHit`
  (params (MyComp :type "PrimitiveComponent Object Reference") (Other :type "Actor Object Reference") (OtherComp :type "PrimitiveComponent Object Reference") (bSelfMoved :type Boolean) (HitLocation :type "Vector Structure") (HitNormal :type "Vector Structure") (NormalImpulse :type "Vector Structure") (Hit :type "HitResult Structure (by ref)"))
  (bind _asrock_bp (cast `/Game/RockBP` Other))
  (if (== (`/Game/RockBP.colorIndex` _asrock_bp) (`self.colorIndex`))
    (set `self.colorIndex` (`KismetMathLibrary.RandomIntegerInRange` 0 8))
    (`MaterialInstanceDynamic.SetVectorParameterValue` (`self.Material`) "Base Color" (`KismetMathLibrary.Conv_ColorToLinearColor` (`|GetArrayItem` (`self.Colors`) (`self.colorIndex`))))))

(event `self.ReceiveBeginPlay`
  (add `self.MaskDispatcher` (delegate `CreateMask`)))

(event `CreateMask`
  (`PrimitiveComponent.SetMaterial` (`self.Sphere`) 0 (`self.Material`)))

(event `self.ReceiveActorBeginOverlap`
  (params (OtherActor :type "Actor Object Reference"))
  (bind _asrock_bp (cast `/Game/RockBP` OtherActor))
  (if (== (`/Game/RockBP.colorIndex` _asrock_bp) (`self.colorIndex`))
    (set `self.colorIndex` (`KismetMathLibrary.RandomIntegerInRange` 0 8))
    (`MaterialInstanceDynamic.SetVectorParameterValue` (`self.Material`) "Base Color" (`KismetMathLibrary.Conv_ColorToLinearColor` (`|GetArrayItem` (`self.Colors`) (`self.colorIndex`))))))

(fn `UserConstructionScript`
  (bind _returnvalue (`KismetMathLibrary.RandomIntegerInRange` 0 8))
  (bind _output_get (set `self.Mesh` (`|GetArrayItem` (`self.Meshes`) _returnvalue)))
  (`StaticMeshComponent.SetStaticMesh` (`self.Sphere`) _output_get)
  (bind _returnvalue_2 (`KismetMaterialLibrary.CreateDynamicMaterialInstance` "/Game/Materials/RockMat_Inst.RockMat_Inst"))
  (bind _output_get_2 (set `self.Material` _returnvalue_2))
  (bind _output_get_3 (set `self.colorIndex` (`KismetMathLibrary.RandomIntegerInRange` 0 8)))
  (`MaterialInstanceDynamic.SetVectorParameterValue` _output_get_2 "Base Color" (`KismetMathLibrary.Conv_ColorToLinearColor` (`|GetArrayItem` (`self.Colors`) _output_get_3)))
  (`PrimitiveComponent.SetMaterial` (`self.Sphere`) 0 (`|GetArrayItem` (`self.MeshMaterials`) _returnvalue)))